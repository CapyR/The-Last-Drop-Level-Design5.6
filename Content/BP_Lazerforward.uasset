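; BP_Lazerforward is a triggered moving actor, named as a laser, that slides its Cube between two target points.
; When a BP_BodyChar overlaps the Box, it prints a debug message and plays a Timeline.
; The Timeline's Z track lerps Cube's world location from TargetCube1 to TargetCube2, without sweep.
; The HasOverlapped guard is only ever set false here, so it does not block retriggering.
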(event OnComponentBeginOverlap(Box)
  (params (OverlappedComponent :type Primitive%20Component%20Object%20Reference) (OtherActor :type Actor%20Object%20Reference) (OtherComp :type Primitive%20Component%20Object%20Reference) (OtherBodyIndex :type Integer) (bFromSweep :type Boolean) (SweepResult :type Hit%20Result%20Structure%20%28by%20ref%29))
  (Utilities|Casting|CastToBP_BodyChar OtherActor)
  (if (not (Variables|Default|GetHasOverlapped?))
    (Development|PrintString "Overlapped")
    (bind _z (Timeline|Timeline Play)
      (:Update
        (Transformation|SetWorldLocation (Variables|Default|GetCube) (Math|Vector|Lerp(Vector) (Transformation|GetWorldLocation (Variables|Default|GetTargetCube%201)) (Transformation|GetWorldLocation (Variables|Default|GetTargetCube%202)) _z) false false)
        (Variables|Default|SetHasOverlapped? false)))))

(event EventBeginPlay)

(event Collision|EventActorBeginOverlap
  (params (OtherActor :type Actor%20Object%20Reference)))

(event EventTick
  (params (DeltaSeconds :type Float%20%28single-precision%29)))

(fn ConstructionScript)