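; Activatable lift platform that moves a static mesh along a multi-stop path, with audio during travel.
; Activation, after a short delay, starts chained timelines that lerp the mesh from start through three targets.
; Later legs trigger from delays on the previous timeline's Update, with FlipFlops alternating play and reverse.
; Once the last leg sets IsLiftOneComplete, activation uses a separate timeline from the final target directly back to start.
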(event EventBeginPlay)

(event Collision|EventActorBeginOverlap
  (params (OtherActor :type Actor%20Object%20Reference)))

(event EventTick
  (params (DeltaSeconds :type Float%20%28single-precision%29)))

(event EventActivate/Deactivate
  (bind _audio (Variables|Default|GetAudio))
  (bind _audio_2 (Variables|Default|GetAudio))
  (bind _audio_3 (Variables|Default|GetAudio))
  (bind _audio_4 (Variables|Default|GetAudio))
  (if (Variables|Default|GetIsLiftOneComplete?)
    (Utilities|FlowControl|Delay 1.0)
    ;[0.15 0.15 0.15 0.5] Going Down
    (Utilities|FlowControl|FlipFlop
      (:A
        (Audio|Components|Audio|Play _audio_3 0.0)
        (bind _z (Timeline|Timeline Play)
          (:Update
            (Transformation|SetWorldLocation (Variables|Default|GetStaticMesh) (Math|Vector|Lerp(Vector) (Transformation|GetWorldLocation (Variables|Default|GetTargetLocation3)) (Transformation|GetWorldLocation (Variables|Default|GetStartLocation)) _z) false false)
            (Variables|Default|SetIsLiftOneComplete? false))
          (:Finished
            (Audio|Components|Audio|Stop (Variables|Default|GetAudio)))))
      (:B
        (Audio|Components|Audio|Play _audio_3 0.0)
        (Timeline|Timeline Reverse)))
    (else
      (Utilities|FlowControl|Delay 1.0)
      (Utilities|FlowControl|FlipFlop
        (:A
          (Audio|Components|Audio|Play _audio 0.0)
          (bind _z_2 (Timeline|UPDown Play)
            (:Update
              (Transformation|SetWorldLocation (Variables|Default|GetStaticMesh) (Math|Vector|Lerp(Vector) (Transformation|GetWorldLocation (Variables|Default|GetStartLocation)) (Transformation|GetWorldLocation (Variables|Default|GetTargetLocation)) _z_2) false false)
              (Utilities|FlowControl|Delay 14.0)
              (Utilities|FlowControl|FlipFlop
                (:A
                  (Audio|Components|Audio|Play _audio_2 0.0)
                  (bind _z_3 (Timeline|Timeline_0 Play)
                    (:Update
                      (Transformation|SetWorldLocation (Variables|Default|GetStaticMesh) (Math|Vector|Lerp(Vector) (Transformation|GetWorldLocation (Variables|Default|GetTargetLocation)) (Transformation|GetWorldLocation (Variables|Default|GetTargetLocation2)) _z_3) false false)
                      (Utilities|FlowControl|Delay 14.0)
                      (Utilities|FlowControl|FlipFlop
                        (:A
                          (Audio|Components|Audio|Play _audio_4 0.0)
                          (bind _z_4 (Timeline|Timeline_1 Play)
                            (:Update
                              (Transformation|SetWorldLocation (Variables|Default|GetStaticMesh) (Math|Vector|Lerp(Vector) (Transformation|GetWorldLocation (Variables|Default|GetTargetLocation2)) (Transformation|GetWorldLocation (Variables|Default|GetTargetLocation3)) _z_4) false false)
                              (Variables|Default|SetIsLiftOneComplete? true))
                            (:Finished
                              (Audio|Components|Audio|Stop (Variables|Default|GetAudio)))))
                        (:B
                          (Audio|Components|Audio|Play _audio_4 0.0)
                          (Timeline|Timeline_1 Reverse))))
                    (:Finished
                      (Audio|Components|Audio|Stop (Variables|Default|GetAudio)))))
                (:B
                  (Audio|Components|Audio|Play _audio_2 0.0)
                  (Timeline|Timeline_0 Reverse))))
            (:Finished
              (Audio|Components|Audio|Stop (Variables|Default|GetAudio)))))
        (:B
          (Audio|Components|Audio|Play _audio 0.0)
          (Timeline|UPDown Reverse))))))

(fn ConstructionScript
  (|CallParentFunction))